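; BP_Button is a button actor that switches off an array of lamps when E is pressed.
; Box overlaps with the third-person character toggle CanPressButton, but the E handler sets it true without checking it.
; The handler calls SwitchOFF on LampsArray entries through the BPI_Switchable interface.
; Any actor overlap also fires the OnPress dispatcher, and IsSwitchON always returns false.
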(event `self.ReceiveActorBeginOverlap`
  (params (OtherActor :type "Actor Object Reference"))
  (`self.OnPress`))

(event `self.Box.OnComponentBeginOverlap`
  (params (OverlappedComponent :type "PrimitiveComponent Object Reference") (OtherActor :type "Actor Object Reference") (OtherComp :type "PrimitiveComponent Object Reference") (OtherBodyIndex :type Integer) (bFromSweep :type Boolean) (SweepResult :type "HitResult Structure (by ref)"))
  (cast `/Game/ThirdPerson/Blueprints/BP_ThirdPersonCharacter` OtherActor)
  (set `self.CanPressButton` true))

(event `self.Box.OnComponentEndOverlap`
  (params (OverlappedComponent :type "PrimitiveComponent Object Reference") (OtherActor :type "Actor Object Reference") (OtherComp :type "PrimitiveComponent Object Reference") (OtherBodyIndex :type Integer))
  (cast `/Game/ThirdPerson/Blueprints/BP_ThirdPersonCharacter` OtherActor)
  (set `self.CanPressButton` false))

(event `Key|E`
  (params (Key :type "Key Structure"))
  (:`Pressed`
    (set `self.CanPressButton` true)
    (for _array_element (`self.LampsArray`)
      (bind _asbpi_switchable (cast `/Game/Tanpleet/BPI_Switchable` _array_element))
      (`/Game/Tanpleet/BPI_Switchable.SwitchOFF` _asbpi_switchable))))

(fn `IsSwitchON`
  (returns (`is on` :type Boolean))
  (return false))

(fn `UserConstructionScript`)